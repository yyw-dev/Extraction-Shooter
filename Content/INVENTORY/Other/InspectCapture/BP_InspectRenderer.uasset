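; Inventory inspect renderer actor that renders a previewed item to a render target through a show-only SceneCapture2D.
; It centers on the attached actors' bounds, attaches to the item mesh and sets spring arm distance from extent or per-item inspect settings.
; Tick interpolates distance and rotation, re-initializing when the attachment count changes.
; It zeroes its spotlight for parented items and self-destroys when the item is destroyed or inspection ends.
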(event Custom|Initialize%20Camera
  (bind _inspecting_settings (Utilities|GetInspectingSettings))
  (bind (_camerainitialrotation _cameraadditionaloffset _useadditionaloffsetasdistance) (Utilities|Struct|BreakInspectCameraInfo _inspecting_settings))
  (Variables|Runtime|SetDefalut%20Intensity (Variables|/Script/Engine.LightComponentBase|GetIntensity (Variables|Components|GetSpotLight)))
  (Utilities|FlowControl|Sequence
    (:then_0
      ;[0.09896 0.09896 0.09896] Get Actor Extent to set camera distance later
      (|AdjustCollisions)
      (bind __actors (Default|GetAttachedActors (Variables|Runtime|GetItem%20To%20Render) true))
      (bind (_center _boxextent) (Collision|GetActorArrayBounds __actors true))
      (Variables|Runtime|SetPivot%20Point _center)
      (Variables|Runtime|SetActorExtent (Class|KismetMathLibrary|VectorGetAbsMax _boxextent))
      (CallFunction|AddShowOnlyActors __actors)
      (Rendering|Components|Light|SetIntensity))
    (:then_1
      ;[0.09896 0.09896 0.09896] Attach Renderer To Preview Item Actor
      (bind _item_to_render (Variables|Runtime|GetItem%20To%20Render)
        (:then
          (Transformation|SetActorLocation (Variables|Runtime|GetPivot%20Point) false false)
          (Transformation|AttachComponentToComponent self (Default|GetItemMesh _item_to_render) "None" "KeepWorld" "KeepRelative" "KeepWorld" false)
          ;[0.09896 0.09896 0.09896] Inspect Settings
          (Transformation|SetActorRelativeRotation _camerainitialrotation)
          (bind _output_get (Variables|/Script/Engine.SpringArmComponent|SetTargetArmLength (Variables|Components|GetSpringArm) (Math|Float|SelectFloat _cameraadditionaloffset (+ _cameraadditionaloffset (* (Variables|Runtime|GetActorExtent) (Variables|Parameters|GetInitial%20Distance%20Multiplier))) _useadditionaloffsetasdistance)))
          (Variables|Runtime|SetRender%20Distance _output_get))
        (:else)))))

(event EventTick
  (params (DeltaSeconds :type Float%20%28single-precision%29))
  ;[0.09896 0.09896 0.09896] Update Camera Distance and Rotation
  (Variables|/Script/Engine.SpringArmComponent|SetTargetArmLength (Variables|Components|GetSpringArm) (|FInterpCameraDistance DeltaSeconds))
  (bind _output_get (Variables|Runtime|SetRotation%20Speed (|RInterpCameraRotationSpeed DeltaSeconds)))
  (Transformation|AddActorLocalRotation _output_get false false)
  (CallFunction|CheckAttachedActors))

(event EventBeginPlay
  (Utilities|IsValid (Variables|Runtime|GetItem%20To%20Render)
    (:Is%20Valid
      (CallFunction|InitializeCamera)
      ;[0.09896 0.09896 0.09896] Bindings
      (|DestroySelfWhenRenderingItemIsDestroyed)
      (|DestroySelfWhenRenderingItemIsNoMoreBeingInspected))))

(fn ConstructionScript)

(fn AddShowOnlyActors
  (params (Array :type Array%20of%20Actor%20Object%20References))
  (for _array_element Array
    (Rendering|SceneCapture|ShowOnlyActorComponents (Variables|Components|GetSceneCaptureComponent2D) _array_element true)))

(fn SetCameraDistance
  (params (New%20Distance :type Float%20%28double-precision%29))
  (Variables|Runtime|SetRender%20Distance New%20Distance))

(fn GetCameraDistance
  (return (Variables|Runtime|GetRender%20Distance)))

(fn StartRendering
  (params (Render%20Size :type Int%20Point%20Structure%20%28by%20ref%29))
  (bind (_x _y) (Utilities|Struct|BreakIntPoint Render%20Size))
  (Components|Activation|Activate (Variables|Components|GetSceneCaptureComponent2D) false)
  (bind _returnvalue (Rendering|CreateRenderTarget2D _x _y "RTF_RGBA16f"))
  (bind _output_get (Variables|/Script/Engine.SceneCaptureComponent2D|SetTextureTarget (Variables|Components|GetSceneCaptureComponent2D) _returnvalue))
  (return _output_get))

(fn StopRendering
  (Components|Activation|Deactivate (Variables|Components|GetSceneCaptureComponent2D)))

(fn CheckAttachedActors
  (bind __actors (Default|GetAttachedActors (Variables|Runtime|GetItem%20To%20Render) true))
  (LocalVariables|SetL%20Length (Utilities|Array|Length __actors))
  (CallFunction|AddShowOnlyActors __actors)
  (if (!= (LocalVariables|GetL%20Length) (Variables|Runtime|GetAttached%20Actors%20Num))
    (Variables|Runtime|SetAttached%20Actors%20Num (LocalVariables|GetL%20Length))
    (CallFunction|InitializeCamera)))

(event Custom|RenderingItemInspectStatus
  (params (BeingInspected :type Boolean))
  (if (not BeingInspected)
    (Actor|DestroyActor)))

(event Custom|Rendering%20Item%20Destroyed
  (params (DestroyedActor :type Actor%20Object%20Reference))
  (Actor|DestroyActor))