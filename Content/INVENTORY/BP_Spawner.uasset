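; Placeable spawner that hides itself at BeginPlay and spawns a configured inventory item on the server.
; The construction script previews the item's mesh and name from its defaults, with a billboard fallback.
; Spawning creates an item object, async-loads and spawns the actor class, fills its ItemInfo and loads sub-items into its inventory.
; Optional flags destroy the spawner afterwards or recenter the item's mesh bounds on the spawner once initialized.
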(event Custom|Spawn%20Item
  (bind _rowname (CallFunction|GetItemIDtoSpawn))
  (Utilities|IsValidName _rowname
    (:Valid
      (Variables|Runtime|SetItem%20Defaults (.ItemDefaults (CallFunction|GetItemDefaultsbyID _rowname)))
      ;[0.09896 0.09896 0.09896] Create Item Object
      (bind _item_object (CallFunction|CreateItemObject (CallFunction|GetItemIDtoSpawn)))
      (Variables|Runtime|SetItem%20Object _item_object)
      ;[0.09896 0.09896 0.09896] Spawn Item & Create its containers
      (|SpawnItemActor)
      (Utilities|FlowControl|Sequence
        (:then_0
          (bind _created_item (CallFunction|CreateItemStructure (CallFunction|GetItemIDtoSpawn) (CallFunction|GetItemAmounttoSpawn) false (Variables|/Game/INVENTORY/Items/BaseBlueprints/_BP_ItemBase._BP_ItemBase_C|GetItem%20Inventory (Variables|Runtime|GetCreated%20Item))))
          (bind _structout (Utilities|Struct|SetmembersinItemInfo _created_item (Variables|Runtime|GetItem%20Object)))
          (Variables|/Game/INVENTORY/Items/BaseBlueprints/_BP_ItemBase._BP_ItemBase_C|SetItem%20Info (Variables|Runtime|GetCreated%20Item) _structout)
          (Utilities|FlowControl|Sequence
            (:then_0
              ;[0.09896 0.09896 0.09896] Load Sub Items Manually
              (for _array_element (Variables|ItemParameters|GetSub%20Items)
                (Default|LoadSubItem (Variables|/Game/INVENTORY/Items/BaseBlueprints/_BP_ItemBase._BP_ItemBase_C|GetItem%20Inventory (Variables|Runtime|GetCreated%20Item)) _array_element false)))
            (:then_1
              (|DestroySelf))))
        (:then_1
          (|FIXITEMPOSITION))))))

(event EventBeginPlay
  ;[0.09896 0.09896 0.09896] Spawn Item on BeginPlay (Only Server)
  (Rendering|SetActorHiddenInGame true)
  (Networking|SwitchHasAuthority
    (:Authority
      (CallFunction|SpawnItem))))

(fn ConstructionScript
  (bind _output_get (LocalVariables|SetL%20Defaults (.ItemDefaults (CallFunction|GetItemDefaultsbyID (CallFunction|GetItemIDtoSpawn)))))
  (Utilities|LoadAssetBlocking (Utilities|Struct|BreakItemActorInfo (.ItemActorInfo (Utilities|Struct|BreakItemDefaults _output_get))))
  (Components|StaticMesh|SetStaticMesh (Variables|Default|GetPreviewMesh) (Utilities|ResolveSoftReference (Utilities|Struct|BreakItemActorInfo (.ItemActorInfo (Utilities|Struct|BreakItemDefaults _output_get)))))
  (Rendering|SetVisibility (Variables|Default|GetBillboard) (not (Utilities|IsValid (Variables|/Script/Engine.StaticMeshComponent|GetStaticMesh (Variables|Default|GetPreviewMesh)))) false)
  (Rendering|Components|TextRender|SetText (Variables|Default|GetTextRender) (.Name (Utilities|Struct|BreakItemDefaults (LocalVariables|GetL%20Defaults)))))

(fn GetItemIDtoSpawn
  (return (Utilities|Struct|BreakDataTableRowHandle (Variables|ItemParameters|GetItem%20ID))))

(fn GetItemAmounttoSpawn
  (return (Math|Integer|SelectInt (Variables|ItemParameters|GetItem%20Amount) 1 (CallFunction|IsStackable (Variables|Runtime|GetItem%20Defaults)))))

(event Custom|OnSpawnedItemInitialized
  (bind _returnvalue (Transformation|GetActorLocation))
  (Transformation|SetWorldLocation (Default|GetItemMesh (Variables|Runtime|GetCreated%20Item)) (+ _returnvalue (- _returnvalue (.Origin (Collision|GetComponentBounds (Default|GetItemMesh (Variables|Runtime|GetCreated%20Item)))))) false true)
  (return))