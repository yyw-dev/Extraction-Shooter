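; Item component that spawns and attaches attachment actors, such as those in an item's equip-slot containers, to the owning item's mesh.
; On authority, it rebuilds attachments after item initialization and, for non-preview items, follows parent inventory slot updates through owner changes.
; Spawning reuses existing actors except for previews, and attachments are destroyed with the owner.
; An initial-only RepNotify waits for the inventory owner, then re-attaches replicated actors to their sockets.
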(event Custom|OnOwnerItemOwnerChanged
  (params (New%20Owner :type Actor%20Object%20Reference))
  ;[0.09896 0.09896 0.09896] Listen Slots
  (Utilities|FlowControl|Sequence
    (:then_0
      (bind _parent_inventory (Variables|Runtime|GetParent%20Inventory)
        (:then
          (EventDispatchers|UnbindEventfromOnSlotUpdatedSERVER _parent_inventory (EventDispatchers|CreateEvent :!event Custom|OnOwnerInventoryAnySlotUpdated))
          (Variables|Runtime|SetParent%20Inventory 0))
        (:else)))
    (:then_1
      (bind _returnvalue (CallFunction|GetParentInventory))
      (Variables|Runtime|SetParent%20Inventory _returnvalue)
      (EventDispatchers|BindEventtoOnSlotUpdatedSERVER (Variables|Runtime|GetParent%20Inventory) (EventDispatchers|CreateEvent :!event Custom|OnOwnerInventoryAnySlotUpdated)))))

(event Custom|OnOwnerInventoryAnySlotUpdated
  (params (Inventory :type Inventory%20Main%20Object%20Reference) (Address :type Slot%20Address%20Structure) (New%20Item :type Item%20Info%20Structure))
  ;[0.09896 0.09896 0.09896] Create Attachment When Item Added To Slot
  (if (== Inventory (Variables|Runtime|GetParent%20Inventory))
    (if (CallFunction|IsOwnAttachmentContainer (CallFunction|GetContainerUID Address))
      (Utilities|IsValidItem New%20Item
        (:Valid
          (CallFunction|CreateAttachmentActor New%20Item true)
          (Default|CallOnItemAddedtoAttachmentSlot New%20Item))
        (:Not%20Valid
          (Default|CallOnItemRemovedfromAttachmentSlot Address))))))

(event Custom|OnOwnerItemDestroyed
  (params (DestroyedActor :type Actor%20Object%20Reference))
  ;[0.09896 0.09896 0.09896] Save Parent Item
  (Actor|DestroyActor (Variables|Runtime|GetAttachment%20Actors)))

(event Custom|OnOwnerItemInitialized
  ;[0.09896 0.09896 0.09896] Load Attachments On Initialize
  (Utilities|FlowControl|DelayUntilNextTick)
  (bind _success (CallFunction|RefreshAttachmentActors :!label _label))
  (|ShouldTryAgain? _success
    (:YES
      (Utilities|FlowControl|DelayUntilNextTick)
      (goto _label))))

(event EventBeginPlay
  ;[0.09896 0.09896 0.09896] Save Parent Item
  (Networking|SwitchHasAuthority
    (:Authority
      (bind _as_bp_item_base (Utilities|Casting|CastTo_BP_ItemBase (Components|GetOwner)))
      (bind _output_get (Variables|Runtime|SetOwner%20Item _as_bp_item_base))
      (Game|AssignOnDestroyed _output_get (delegate Custom|OnOwnerItemDestroyed))
      (bind _returnvalue (CallFunction|GetParentInventory))
      (Variables|Runtime|SetParent%20Inventory _returnvalue)
      ;[0.09896 0.09896 0.09896] Load Attachments On Initialize
      (EventDispatchers|AssignOnItemInitialized (Variables|Runtime|GetOwner%20Item) (delegate Custom|OnOwnerItemInitialized))
      (if (not (Default|IsPreviewActor (Variables|Runtime|GetOwner%20Item)))
        (EventDispatchers|AssignOnOwnerChanged (Variables|Runtime|GetOwner%20Item) (delegate Custom|OnOwnerItemOwnerChanged))))))

(fn CreateAttachmentActor
  (params (Attachment%20Item :type Item%20Info%20Structure) (Auto%20Attach :type Boolean))
  (bind _itemdefaults (CallFunction|GetItemDefaults Attachment%20Item))
  (bind _itemactorinfo (Utilities|Struct|BreakItemDefaults _itemdefaults))
  (bind (_itemactorclass _equipsocket) (Utilities|Struct|BreakItemActorInfo _itemactorinfo))
  ;[0.09896 0.09896 0.09896] Should item be spawned on attach
  (LocalVariables|SetL%20Attachment%20Defaults (CallFunction|GetItemDefaults Attachment%20Item))
  (if (|ShouldActorBeSpawned)
    (Utilities|FlowControl|Sequence
      (:then_0
        (Utilities|FlowControl|Sequence
          (:then_0
            ;[0.09896 0.09896 0.09896] Spawn Attachment Actor
            (LocalVariables|SetL%20Socket _equipsocket)
            (|ShouldUseExistingItemActor
              (:Yes
                (LocalVariables|SetL%20Attachment%20Actor (CallFunction|GetItemActor Attachment%20Item)))
              (:No
                (bind _returnvalue (Utilities|LoadClassAssetBlocking _itemactorclass))
                (bind _as_bp_item_base (Utilities|Casting|CastTo_BP_ItemBaseClass _returnvalue))
                (bind _returnvalue_2 (Game|SpawnActorfromClass _as_bp_item_base (Math|Transform|MakeTransform "500.000000,500.000000,500.000000" "0, 0, 0" "1.000000,1.000000,1.000000") "AdjustIfPossibleButAlwaysSpawn" (Variables|Runtime|GetOwner%20Item) Attachment%20Item (Default|IsPreviewActor (Variables|Runtime|GetOwner%20Item)) 0))
                (bind _output_get (LocalVariables|SetL%20Attachment%20Actor _returnvalue_2))
                (Game|BindEventtoOnDestroyed _output_get (EventDispatchers|CreateEvent :!event RemoveAttachmentfromArray))
                (Default|CallOnCreatedAttachmentActor _output_get))))
          (:then_1
            ;;[0.09896 0.09896 0.09896] Attach it
            (if Auto%20Attach
              (Default|AttachItemtoComponent (LocalVariables|GetL%20Attachment%20Actor) (Default|GetItemMesh (Variables|Runtime|GetOwner%20Item)) (LocalVariables|GetL%20Socket))))))
      (:then_1
        (Utilities|Array|AddUnique (Variables|Runtime|GetAttachment%20Actors) (LocalVariables|GetL%20Attachment%20Actor))
        (return (LocalVariables|GetL%20Attachment%20Actor))))))

(fn RefreshAttachmentActors
  (if (or (Ability|HasAuthority (Components|GetOwner)) (Default|IsPreviewActor (Variables|Runtime|GetOwner%20Item))) ; This function only be called by server,\nor client if item is preview actor.
    ;[0.09896 0.09896 0.09896] Destroy Existing Attachment Actors
    (bind __actors (Default|GetAttachedActors (Variables|Runtime|GetOwner%20Item) false))
    (Actor|DestroyActor __actors)
    ;[0.09896 0.09896 0.09896] Create Attachments
    (for _array_element (Utilities|Struct|BreakItemInfo (Variables|/Game/INVENTORY/Items/BaseBlueprints/_BP_ItemBase._BP_ItemBase_C|GetItem%20Info (Variables|Runtime|GetOwner%20Item)))
      (bind _output_get (LocalVariables|SetL%20Container (Default|GetContainer(copy)byUID (Variables|Runtime|GetParent%20Inventory) _array_element))) ; Equipslot Container
      (Utilities|IsValidContainer _output_get
        (:valid
          (if (Utilities|Array|IsNotEmpty (Utilities|Struct|BreakContainerInfo _output_get))
            (CallFunction|CreateAttachmentActor (Utilities|Array|Get(acopy) (Utilities|Struct|BreakContainerInfo _output_get)) true)))
        (:NotValid
          (return false))))
    (Default|CallOnAttachmentsRefreshed)
    (return true)))

(fn AreAllAttachmentsInitialized
  (for _array_element (Variables|Runtime|GetAttachment%20Actors)
    (if (not (Default|IsInitialized _array_element))
      (return false)))
  (return true))

(fn RemoveAttachmentfromArray
  (params (Actor :type Actor%20Object%20Reference))
  (bind _as_bp_item_base (Utilities|Casting|CastTo_BP_ItemBase Actor))
  (Utilities|Array|RemoveItem (Variables|Runtime|GetAttachment%20Actors) _as_bp_item_base))

(fn IsOwnAttachmentContainer
  (params (Container%20UID :type Integer%20%28by%20ref%29))
  (Utilities|FlowControl|Sequence
    (:then_0
      (if (Utilities|Array|ContainsItem (Utilities|Struct|BreakItemInfo (Variables|/Game/INVENTORY/Items/BaseBlueprints/_BP_ItemBase._BP_ItemBase_C|GetItem%20Info (Variables|Runtime|GetOwner%20Item))) Container%20UID)
        (if (!= (Utilities|Struct|BreakContainerInfo (Default|GetContainer(copy)byUID (Variables|Runtime|GetParent%20Inventory) Container%20UID)) (Utilities|GetGeneralInventorySlotType))
          (return true))))
    (:then_1
      (return false))))

(fn GetOwnerItem
  (bind _as_bp_item_base (Utilities|Casting|CastTo_BP_ItemBase (Components|GetOwner)))
  (return _as_bp_item_base))

(fn GetParentInventory
  (bind _returnvalue (Components|GetOwner))
  (bind _returnvalue_2 (Components|GetOwner _returnvalue))
  (Utilities|IsValid _returnvalue_2
    (:Is%20Valid
      (return (Actor|GetComponentbyClass _returnvalue_2 "/Game/INVENTORY/Core/Inventory__Main.Inventory__Main_C")))
    (:Is%20Not%20Valid
      (return (Actor|GetComponentbyClass _returnvalue "/Game/INVENTORY/Core/Inventory__Main.Inventory__Main_C")))))

(fn FindAttachmentonContainer
  (params (Attachment%20Container%20Type :type Gameplay%20Tag%20Structure))
  (bind _returnvalue (CallFunction|GetParentInventory))
  (for _array_element (Utilities|Struct|BreakItemInfo (Variables|/Game/INVENTORY/Items/BaseBlueprints/_BP_ItemBase._BP_ItemBase_C|GetItem%20Info (Variables|Runtime|GetOwner%20Item)))
    (bind _output_get (LocalVariables|SetL%20Container (Default|GetContainer(copy)byUID _returnvalue _array_element)))
    (if (== Attachment%20Container%20Type (.ContainerType (Utilities|Struct|BreakContainerInfo _output_get)))
      (if (Utilities|Array|IsNotEmpty (.Items (Utilities|Struct|BreakContainerInfo _output_get)))
        (return (Utilities|Array|Get(acopy) (.Items (Utilities|Struct|BreakContainerInfo _output_get)))))))
  (return ""))

(event Custom|OnRep_Attachment%20Actors
  (Utilities|FlowControl|DoOnce false
    (:Completed
      (Utilities|IsValid (Components|GetOwner (Variables|Runtime|GetParent%20Inventory)) :!label _label
        (:Is%20Valid
          (Utilities|FlowControl|Delay 0.2)
          (for _array_element (Variables|Runtime|GetAttachment%20Actors)
            (Utilities|IsValid _array_element
              (:Is%20Valid
                (Default|AttachItemtoComponent _array_element (Default|GetItemMesh (CallFunction|GetOwnerItem)) (|GetEquipSocket _array_element))))))
        (:Is%20Not%20Valid
          (Utilities|FlowControl|DelayUntilNextTick)
          (goto _label))))))