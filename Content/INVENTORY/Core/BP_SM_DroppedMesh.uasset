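; Static mesh component on an item that stands in for the item's skeletal main mesh as a physics-simulated dropped mesh.
; The IsEnabled RepNotify swaps visibility, physics and Visibility-trace blocking, then registers the active mesh as the item's mesh component reference.
; Disabling snaps it back to the item root and restores the original mesh.
; Each toggle can also send a trace-leave message to the owner where cosmetic events run.
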(event EventBeginPlay
  ;[0.09896 0.09896 0.09896] Save owner item variables at beginplay.
  (bind _as_bp_item_base (Utilities|Casting|CastTo_BP_ItemBase (Components|GetOwner)))
  (bind _output_get (Variables|Runtime|SetParent%20Item _as_bp_item_base))
  (bind _mesh_component (Default|FindItemMeshComponent _output_get))
  (Variables|Runtime|SetParent%20Item%20Main%20Mesh _mesh_component))

(fn OnRepIsEnabled
  (bind _mesh (CallFunction|GetParentItemMainMesh))
  (bind _mesh_2 (CallFunction|GetParentItemMainMesh))
  ;[0.09896 0.09896 0.09896] Set self as Main Mesh of item, and overwrite physics and collisions.
  (Utilities|FlowControl|Sequence
    (:then_0
      (if (Variables|Runtime|GetIs%20Enabled)
        (Utilities|FlowControl|Sequence
          (:then_0
            (Rendering|SetVisibility true false)
            (Rendering|SetVisibility _mesh_2 false false)
            (Physics|SetSimulatePhysics _mesh_2 false)
            (Physics|SetSimulatePhysics true)
            (Collision|SetCollisionResponsetoChannel "ECC_Visibility" "ECR_Block"))
          (:then_1
            (Default|SetItemMeshComponentReference (CallFunction|GetParentItem) self) ; Set self as Main Mesh Component Reference of parent item.
          ))
        (else
          (Rendering|SetVisibility false false)
          (Physics|SetSimulatePhysics false)
          (Transformation|AttachComponentToComponent (Variables|/Script/Engine.Actor|GetRootComponent (CallFunction|GetParentItem)) "None" "SnapToTarget" "SnapToTarget" "SnapToTarget" false)
          (Rendering|SetVisibility _mesh true false)
          (Default|SetItemMeshComponentReference (CallFunction|GetParentItem) _mesh) ; Set old mesh as Main Mesh Component Reference of parent item.
          (Collision|SetCollisionResponsetoChannel "ECC_Visibility" "ECR_Ignore"))))
    (:then_1
      (Networking|CanExecuteCosmeticEvents
        (:True
          (Utilities|IsValid (CallFunction|GetLocalInventoryComponent)
            (:Is%20Valid
              (Class|BPIInteractable|OnTraceLeave(Message) (Components|GetOwner)))))))))

(fn GetParentItem
  (bind _parent_item (Variables|Runtime|GetParent%20Item)
    (:then
      (return _parent_item))
    (:else
      (bind _as_bp_item_base (Utilities|Casting|CastTo_BP_ItemBase (Components|GetOwner)))
      (bind _output_get (Variables|Runtime|SetParent%20Item _as_bp_item_base))
      (return _output_get))))

(fn GetParentItemMainMesh
  ;[0.09896 0.09896 0.09896 1 15] Return Parent Item's Skeletal Mesh.
  (bind _parent_item_main_mesh (Variables|Runtime|GetParent%20Item%20Main%20Mesh)
    (:then
      (return _parent_item_main_mesh))
    (:else
      (bind _mesh_component (Default|FindItemMeshComponent (CallFunction|GetParentItem)))
      (return _mesh_component))))