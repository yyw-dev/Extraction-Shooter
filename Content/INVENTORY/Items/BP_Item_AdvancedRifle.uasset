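; Inventory rifle item with automatic fire, aim-down-sights, and magazine and silencer attachments.
; A rate-limited firing gate spends magazine bullets, line-traces along the owner's aim for point damage, spawns trails and applies recoil.
; Fire attempts update the ammo widget and trigger client-side sound and muzzle flash events, adjusted for the silencer.
; Reload uses montage notifies to move magazine items between the inventory and the rifle's magazine container.
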(event EventSetSilencerReference
  (params (New%20Value :type Boolean))
  ;[0.09896 0.09896 0.09896] Attachment parameters
  (Variables|Runtime|SetHas%20Silencer New%20Value))

(event EventSetMagazineReference
  (params (Magazine :type BP%20Item%20Magazine%20Base%20Object%20Reference))
  ;[0.09896 0.09896 0.09896] Attachment parameters
  (Variables|Runtime|SetMagazine%20Reference Magazine))

(event EventBeginPlay
  ;[0.09896 0.09896 0.09896] BeginPlay
  (|CallParentFunction)
  (EventDispatchers|AssignOnFireAttempt (EventDispatchers|CreateEvent :!event Custom|Fire%20Attempt))
  (|SetAmmoUIReference))

(fn ConstructionScript
  (|CallParentFunction))

(fn FireTrace
  (params (Start :type Vector) (End :type Vector))
  (bind _outhit (Collision|LineTraceByChannel Start End "TraceTypeQuery1" false (Utilities|Array|MakeArray (Components|GetOwner) self) (select (Variables|/Game/INVENTORY/Core/Inventory__Main.Inventory__Main_C|GetDebug%20Mode (Variables|Default|GetOwner%20Inventory)) "ForDuration" "None") false "(R=0.965850,G=0.000000,B=1.000000,A=1.000000)" "(R=0.000000,G=1.000000,B=0.000000,A=1.000000)" 3.0))
  (return _outhit))

(fn HandleTrace
  (params (Hit%20Result :type Hit%20Result%20Structure))
  (bind (_bblockinghit _binitialoverlap _time _distance _location _impactpoint _normal _impactnormal _physmat _hitactor _hitcomponent _hitbonename _bonename _hititem _elementindex _faceindex _tracestart _traceend) (Collision|BreakHitResult Hit%20Result))
  (Utilities|FlowControl|Sequence
    (:then_0
      (if _bblockinghit
        (Game|Damage|ApplyPointDamage _hitactor (Variables|WeaponParameters|FireTrace|GetDamage%20Per%20Trace) (Math|Vector|GetUnitDirection(Vector) _tracestart _impactpoint) Hit%20Result (Pawn|GetController (.AsPawn (Utilities|Casting|CastToPawn (Components|GetOwner)))) self)))
    (:then_1
      (Game|SpawnActorfromClass "/Game/INVENTORY/Other/VFX/Firetrail/BP_FireTrail.BP_FireTrail_C" (Math|Transform|MakeTransform (Transformation|GetSocketLocation (CallFunction|GetItemMesh) (Variables|WeaponParameters|FireTrace|GetMuzzle%20Socket))) "AlwaysSpawn" 0 (* (Math|Random|RandomUnitVectorinConeinDegrees (Math|Vector|GetUnitDirection(Vector) _tracestart _traceend) 1.0) 2e+04) 0))))

(fn GetFireTracePoints
  (bind _returnvalue (Components|GetOwner))
  (Utilities|IsValid _returnvalue
    (:Is%20Valid
      (bind (_start_location _forward_vector) (Class|BPIInteractable|GetTracePoint(Message) _returnvalue))
      (return (Class|KismetMathLibrary|ProjectPointontoPlane (+ _start_location (* _forward_vector (Variables|WeaponParameters|FireTrace|GetBullet%20Trace%20Length))) (Transformation|GetSocketLocation (CallFunction|GetItemMesh) (Variables|WeaponParameters|FireTrace|GetMuzzle%20Socket)) _forward_vector) (+ _start_location (* _forward_vector (Variables|WeaponParameters|FireTrace|GetBullet%20Trace%20Length)))))))

(fn ToggleAmmoUI
  (params (Show :type Boolean))
  (Utilities|FlowControl|Sequence
    (:then_0
      (if Show
        (CallFunction|UpdateAmmoUI)))
    (:then_1
      (bind _ammo_ui (Variables|Runtime|GetAmmo%20UI)
        (:then
          (Default|ToggleInfoVisibility _ammo_ui Show))
        (:else)))))

(fn UpdateAmmoUI
  (bind _ammo_ui (Variables|Runtime|GetAmmo%20UI)
    (:then
      (bind _magazine_reference (Variables|Runtime|GetMagazine%20Reference)
        (:then
          (Default|UpdateAmmoCount _ammo_ui (Default|GetBulletCount _magazine_reference)))
        (:else)))
    (:else)))

(fn GetMagazineContainerUID
  (Utilities|IsValidID (Variables|Runtime|GetMagazine%20Container%20Index)
    (:valid
      (return (Utilities|Array|Get(acopy) (Utilities|Struct|BreakItemInfo (Variables|Default|GetItem%20Info)) (Variables|Runtime|GetMagazine%20Container%20Index))))
    (:NotValid
      (for (_array_element _array_index) (Utilities|Struct|BreakItemInfo (Variables|Default|GetItem%20Info))
        (if (== (Utilities|Struct|BreakContainerInfo (Default|GetContainer(copy)byUID (Variables|Default|GetOwner%20Inventory) _array_element)) "(TagName=\"Attachments.Magazine\")")
          (bind _output_get (Variables|Runtime|SetMagazine%20Container%20Index _array_index))
          (return (Utilities|Array|Get(acopy) (Utilities|Struct|BreakItemInfo (Variables|Default|GetItem%20Info)) _output_get)))))))

(event Custom|Play%20Fire%20Sound%20CLIENTS
  (params (VolumeMultiplier :type Float%20%28single-precision%29) (PitchMultiplier :type Float%20%28single-precision%29) (Location :type Vector))
  (Audio|PlaySoundatLocation (Variables|WeaponParameters|Sounds|GetFire%20Sound) Location "0, 0, 0" VolumeMultiplier PitchMultiplier 0.0 0 0 0 0))

(event Custom|Play%20Out%20of%20Ammo%20Sound%20CLIENTS
  (params (Location :type Vector))
  (Audio|PlaySoundatLocation (Variables|WeaponParameters|Sounds|GetOut%20of%20Ammo%20Sound) Location "0, 0, 0" 1.0 1.0 0.0 0 0 0 0))

(event Custom|Activate%20Muzzle%20Flash%20CLIENTS
  (Components|Activation|Activate (Variables|Default|GetParticleSystem) true))

(event Custom|Recoil%20CLIENT
  ;[0.04761 0.04076 0.09896] Recoil
  (bind _combat_component (Utilities|GetOwnerCombat)
    (:Is%20Valid
      (Pawn|Input|AddControllerPitchInput (Variables|/Game/INVENTORY/Core/CombatComponent.CombatComponent_C|GetOwner%20Character _combat_component) (* (Math|Float|Absolute(Float) (Variables|WeaponParameters|Recoil|GetY%20Recoil)) -1.0))
      (Pawn|Input|AddControllerYawInput (Variables|/Game/INVENTORY/Core/CombatComponent.CombatComponent_C|GetOwner%20Character _combat_component) (Math|Random|RandomFloatinRange (* (Variables|WeaponParameters|Recoil|GetX%20Recoil) -1.0) (Variables|WeaponParameters|Recoil|GetX%20Recoil))))))

(event Custom|Send%20Hit%20Feedback%20CLIENT
  (params (Sound :type Sound%20Base%20Object%20Reference) (Hitmarker%20Color :type Linear%20Color%20Structure))
  (bind _combat_component (Utilities|GetOwnerCombat)
    (:Is%20Valid
      (Default|HitFeedback _combat_component Hitmarker%20Color)
      (Audio|PlaySound2D Sound 1.0 1.0 0.0 0 0 false))))

(event EventSendHitFeedback
  (params (Sound :type Sound%20Base%20Object%20Reference) (Hitmarker%20Color :type Linear%20Color%20Structure))
  (CallFunction|SendHitFeedbackCLIENT Sound Hitmarker%20Color))

(event EventPrimaryUse
  ;[0.09896 0.09896 0.09896] Fire
  (Utilities|FiringGate :!label _label
    (:Fire%20Loop
      (bind _magazine_reference (Variables|Runtime|GetMagazine%20Reference)
        (:then
          (Default|CallOnFireAttempt)
          (if (Default|HasBullet _magazine_reference)
            (Utilities|FlowControl|Sequence
              (:then_0
                (Utilities|SetIsFiring true)
                (Default|AddBulletCount (Variables|Runtime|GetMagazine%20Reference) -1)
                (bind (_start _end) (CallFunction|GetFireTracePoints))
                (bind _outhit (CallFunction|FireTrace _start _end))
                (CallFunction|HandleTrace _outhit)
                (CallFunction|RecoilCLIENT)))
            (else
              (goto _label Stop%20Fire))))
        (:else)))
    (:Stopped
      (Utilities|SetIsFiring false))))

(event EventStopPrimaryUsing
  ;[0.09896 0.09896 0.09896] Fire
  (Utilities|FiringGate) ; enters at Stop Fire
)

(event EventSecondaryUse
  ;[0.09896 0.09896 0.09896] ADS
  (bind _combat_component (Utilities|GetOwnerCombat)
    (:Is%20Valid
      (if (not (Variables|/Game/INVENTORY/Core/CombatComponent.CombatComponent_C|GetIs%20Sprinting _combat_component))
        (Variables|/Game/INVENTORY/Core/CombatComponent.CombatComponent_C|SetIs%20ADS _combat_component true)
        (Default|AddCameraOffset _combat_component (Variables|WeaponParameters|GetADS%20Camera%20Offset))
        (CallFunction|ToggleAmmoUI (Utilities|IsValid (Variables|Runtime|GetMagazine%20Reference)))))))

(event EventStopSecondaryUsing
  ;[0.09896 0.09896 0.09896] ADS
  (bind _combat_component (Utilities|GetOwnerCombat)
    (:Is%20Valid
      (Variables|/Game/INVENTORY/Core/CombatComponent.CombatComponent_C|SetIs%20ADS _combat_component false)
      (Default|ResetCameraDistance _combat_component)
      (Variables|Runtime|GetAmmo%20UI
        (:then
          (CallFunction|ToggleAmmoUI false))
        (:else)))))

(event EventReload
  ;[0.09896 0.09896 0.09896] Reload
  (Utilities|GetOwnerCombat
    (:Is%20Valid
      (Utilities|IsValidItem (Default|GetItem(copy)byUID (Variables|Default|GetOwner%20Inventory) (Utilities|Struct|MakeSlotAddress (CallFunction|GetMagazineContainerUID) 0)) ; Is there already a magazine on slot
        (:Valid
          (bind (_found _space_address _rotated) (Default|FindSpaceforItem (Variables|Default|GetOwner%20Inventory) (Utilities|Struct|BreakDataTableRowHandle (Variables|WeaponParameters|GetMagazine%20Item%20ID)) 1 true "(GameplayTags=((TagName=\"Attachments.Magazine\")))")) ; Find space to remove existing magazine from slot
          (if _found
            (bind (_results _found_amount) (Default|FindItem (Variables|Default|GetOwner%20Inventory) (Utilities|Struct|BreakDataTableRowHandle (Variables|WeaponParameters|GetMagazine%20Item%20ID)) -1 false :!label _label)) ; Find new magazine item.
            (if (> _found_amount 0)
              (bind _notifyname (Animation|Montage|PlayMontage (Variables|/Script/Engine.Character|GetMesh (Variables|/Game/INVENTORY/Core/CombatComponent.CombatComponent_C|GetOwner%20Character (Variables|Default|GetOwner%20Combat))) (Variables|WeaponParameters|Montages|GetReload%20Montage))
                (:OnNotifyBegin
                  (switch string (Utilities|String|ToString(Name) _notifyname)
                    (:MagOut
                      (Default|RepositionItem (Variables|Default|GetOwner%20Inventory) (Utilities|Struct|MakeSlotAddress (CallFunction|GetMagazineContainerUID)) _space_address 1 _rotated) ; Remove existing magazine from slot
                    )
                    (:MagIn
                      (bind _array_element (Utilities|Array|ForEachLoopwithBreak _results :!label _label_2) ; Iterate all found magazine items
                        (:LoopBody
                          (if (not (Utilities|Array|ContainsItem (Utilities|Struct|BreakItemInfo (Variables|Default|GetItem%20Info)) (CallFunction|GetContainerUID (Utilities|Struct|BreakFindResult _array_element)))) ; Ignore it if it is already equipped one
                            (bind _success (Default|RepositionItem (Variables|Default|GetOwner%20Inventory) (Utilities|Struct|BreakFindResult _array_element) (Utilities|Struct|MakeSlotAddress (CallFunction|GetMagazineContainerUID)) 1 false)) ; Move new magazine to magazine container.
                            (if _success
                              (goto _label_2 Break))))))))))))
        (:Not%20Valid
          (goto _label))))))

(event Custom|Fire%20Attempt
  (bind _returnvalue (Transformation|GetActorLocation))
  ;[0.09896 0.09896 0.09896] Fire Attempt
  (CallFunction|UpdateAmmoUI)
  (bind _magazine_reference (Variables|Runtime|GetMagazine%20Reference)
    (:then
      (if (Default|HasBullet _magazine_reference)
        (Utilities|FlowControl|Sequence
          (:then_0
            ;;[0.09896 0.09896 0.09896] Muzzle Flash
            (if (not (Variables|Runtime|GetHas%20Silencer))
              (CallFunction|ActivateMuzzleFlashCLIENTS)))
          (:then_1
            ;;[0.09896 0.09896 0.09896] Fire Sound
            ;;;[0.09896 0.09896 0.09896 1 12] You can remake the silencer sound logic. This is an example.
            (if (Variables|Runtime|GetHas%20Silencer)
              (CallFunction|PlayFireSoundCLIENTS 0.3 1.0 _returnvalue)
              (else
                (CallFunction|PlayFireSoundCLIENTS 1.0 0.5 _returnvalue)))))
        (else
          (Utilities|IsReloading
            (:False
              (CallFunction|PlayOutOfAmmoSoundCLIENTS (Transformation|GetActorLocation)))))))
    (:else)))