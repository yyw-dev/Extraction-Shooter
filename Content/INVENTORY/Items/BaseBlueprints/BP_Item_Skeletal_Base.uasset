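; Base Blueprint for skeletal inventory items that use a separate BP_SM_DroppedMesh component for their dropped state.
; It overrides UpdateCollisionandPhysics to enable that component only while the item has no owner, provided a static mesh is assigned.
; It then calls the parent collision and physics update, and the construction script simply defers to the parent.
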(event EventUpdateCollisionandPhysics
  ;[0.09896 0.09896 0.09896] Override physics event via BP_SM_DroppedMesh component.
  (Utilities|FlowControl|Sequence
    (:then_0
      (Utilities|IsValid (Variables|/Script/Engine.StaticMeshComponent|GetStaticMesh (Variables|Default|GetBP_SM_DroppedMesh))
        (:Is%20Valid
          (Variables|/Game/INVENTORY/Core/BP_SM_DroppedMesh.BP_SM_DroppedMesh_C|SetIs%20Enabled (Variables|Default|GetBP_SM_DroppedMesh) (not (Variables|Default|GetHas%20Owner))))))
    (:then_1
      (|CallParentFunction))))

(fn ConstructionScript
  (|CallParentFunction))