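; Base Blueprint for holdable inventory item actors that drive their owner's animation state while held.
; Attaching to the item's designated socket applies AnimStateOnHeld through the owner's CombatComponent, while other sockets or detaching reset it if the item is still held.
; Changing owner resets the previous owner's anim state, clears its HeldItem if it is this item, then re-caches the combat and Inventory_Equipper components.
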(event EventDetachfromOwner
  (|CallParentFunction)
  (if (CallFunction|IsHeld)
    (bind _owner_combat (Variables|Runtime|GetOwner%20Combat)
      (:then
        (Default|SetAnimState _owner_combat "NewEnumerator0"))
      (:else))))

(event EventAttachItemtoComponent
  (params (Component :type Scene%20Component%20Object%20Reference) (SocketName :type Name :default "None"))
  (|CallParentFunction Component SocketName)
  (if (== (Default|GetActorSocket (CallFunction|GetItemObject (Variables|Default|GetItem%20Info)) true) SocketName)
    (bind _owner_combat (Variables|Runtime|GetOwner%20Combat)
      (:then
        (Default|SetAnimState _owner_combat (Variables|Parameters|GetAnim%20State%20On%20Held)))
      (:else))
    (elif (CallFunction|IsHeld)
      (bind _owner_combat_2 (Variables|Runtime|GetOwner%20Combat)
        (:then
          (Default|SetAnimState _owner_combat_2 "NewEnumerator0"))
        (:else)))))

(fn ConstructionScript
  (|CallParentFunction))

(fn SetReferences
  (bind _returnvalue (Components|GetOwner))
  (if (CallFunction|HasValidOwner)
    (Variables|Runtime|SetOwner%20Combat (Actor|GetComponentbyClass _returnvalue "/Game/INVENTORY/Core/CombatComponent.CombatComponent_C"))
    (Variables|Runtime|SetOwner%20Inventory (Actor|GetComponentbyClass _returnvalue "/Game/INVENTORY/Core/Inventory_Equipper.Inventory_Equipper_C"))))

(fn IsHeld
  (bind _owner_inventory (Variables|Runtime|GetOwner%20Inventory)
    (:then
      (return (Default|IsHeldItem _owner_inventory self)))
    (:else
      (return false))))

(fn SetItemActorOwner
  (params (New%20Owner :type Actor%20Object%20Reference))
  (|CallParentFunction New%20Owner)
  (Utilities|FlowControl|Sequence
    (:then_0
      ;[0.09896 0.09896 0.09896] Reset Old Owner Anim State
      (Utilities|FlowControl|Sequence
        (:then_0
          (bind _owner_combat (Variables|Runtime|GetOwner%20Combat)
            (:then
              (Default|SetAnimState _owner_combat "NewEnumerator0") ; Reset locomotion to default
            )
            (:else)))
        (:then_1
          (bind _owner_inventory (Variables|Runtime|GetOwner%20Inventory)
            (:then
              (if (Default|IsHeldItem _owner_inventory self)
                (Variables|/Game/INVENTORY/Core/Inventory_Equipper.Inventory_Equipper_C|SetHeld%20Item _owner_inventory 0)))
            (:else)))))
    (:then_1
      (CallFunction|SetReferences))))

(fn IsOwnerInventory
  (params (Inventory :type Object%20Object%20Reference))
  (return (== Inventory (Variables|Runtime|GetOwner%20Inventory))))