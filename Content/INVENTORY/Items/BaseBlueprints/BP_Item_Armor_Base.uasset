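; Base Blueprint for armor items that intercepts point damage and passes it on to the owning Pawn.
; Incoming damage is multiplied by DamageReduction as a percentage, so the value is the share that gets through, then reapplied to the owner with the owner's controller as instigator.
; The damage causer then receives a hit feedback message carrying the armor's sound and hitmarker color.
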(event Game|Damage|EventPointDamage
  (params (Damage :type Float%20%28single-precision%29) (DamageType :type Damage%20Type%20Object%20Reference) (HitLocation :type Vector :default "0, 0, 0") (HitNormal :type Vector :default "0, 0, 0") (HitComponent :type Primitive%20Component%20Object%20Reference) (BoneName :type Name :default "None") (ShotFromDirection :type Vector :default "0, 0, 0") (InstigatedBy :type Controller%20Object%20Reference) (DamageCauser :type Actor%20Object%20Reference) (HitInfo :type Hit%20Result%20Structure%20%28by%20ref%29))
  (bind _aspawn (Utilities|Casting|CastToPawn (Components|GetOwner)))
  (Game|Damage|ApplyPointDamage (Components|GetOwner) (CallFunction|CalculateNewDamage Damage) ShotFromDirection HitInfo (Pawn|GetController _aspawn) DamageCauser)
  (Class|BPIDamageFeedback|SendHitFeedback(Message) DamageCauser (Variables|Default|GetHit%20Feedback%20Sound) (Variables|Default|GetHit%20Feedback%20Color)))

(fn ConstructionScript
  (|CallParentFunction))

(fn CalculateNewDamage
  (params (Damage :type Float%20%28double-precision%29))
  (return (* Damage (/ (Variables|Default|GetDamage%20Reduction) 1e+02))))