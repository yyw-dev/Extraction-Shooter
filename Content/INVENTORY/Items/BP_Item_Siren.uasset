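; BP_Item_Siren is an inventory item that acts as a flashing siren light while it has a valid owner.
; Setting the item's owner updates IsEnabled, whose RepNotify drives the point light's intensity and a looping timer.
; The timer uses a negative start delay to cancel the first wait, and a FlipFlop alternates between the primary and secondary colors.
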(event Custom|Toggle%20Siren
  (params (Enable :type Boolean))
  (Variables|Runtime|SetIs%20Enabled Enable))

(event Custom|Color%20Switch%20Event
  (bind _pointlight (Variables|Default|GetPointLight))
  (Utilities|FlowControl|FlipFlop
    (:A
      (Rendering|Components|Light|SetLightColor _pointlight (Variables|Parameters|GetPrimary%20Color) true))
    (:B
      (Rendering|Components|Light|SetLightColor _pointlight (Variables|Parameters|GetSecondary%20Color) true))))

(fn ConstructionScript
  (|CallParentFunction))

(fn OnRepIsEnabled
  (bind _color_switch_interval (Variables|Parameters|GetColor%20Switch%20Interval))
  (if (Variables|Runtime|GetIs%20Enabled)
    (bind _returnvalue (Utilities|Time|SetTimerbyEvent (EventDispatchers|CreateEvent :!event Custom|Color%20Switch%20Event) _color_switch_interval true (* _color_switch_interval -1.0)))
    (Variables|Runtime|SetColor%20Switch%20Timer _returnvalue)
    (Rendering|Components|Light|SetIntensity (Variables|Default|GetPointLight) (Variables|Parameters|GetSiren%20Default%20Intensity))
    (else
      (Utilities|Time|ClearandInvalidateTimerbyHandle (Variables|Runtime|GetColor%20Switch%20Timer))
      (Rendering|Components|Light|SetIntensity (Variables|Default|GetPointLight) 0.0))))

(fn SetItemActorOwner
  (params (New%20Owner :type Actor%20Object%20Reference))
  (|CallParentFunction New%20Owner)
  (CallFunction|ToggleSiren (Utilities|IsValid New%20Owner)))