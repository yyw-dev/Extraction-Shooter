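; Flashlight inventory item that toggles a light on primary use, powered by battery items in its attachment slots.
; A looping timer, paused while off, drains the active battery; when depleted or removed, it searches its own containers for another charged one, otherwise going dark.
; RepNotify variables drive light intensity and hide the actor when unequipped, since it lacks a secondary socket.
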(event OnItemAddedtoAttachmentSlot(BP_AttachmentHandler)
  (params (Added%20Item :type Item%20Info%20Structure))
  (bind (_itemid _itemobject) (Utilities|Struct|BreakItemInfo Added%20Item))
  ;[0.09896 0.09896 0.09896] On Attach Battery
  (if (not (CallFunction|IsPreviewActor))
    (if (== _itemid (Utilities|Struct|BreakDataTableRowHandle (Variables|Parameters|GetBattery%20Item))) ; Is it battery?
      (Utilities|IsValid (Variables|Runtime|GetActive%20Battery) ; Is there already battery attached?
        (:Is%20Valid
          (if (Default|IsPercentZero (Variables|Runtime|GetActive%20Battery)) ; is already attached battery 0 percent?
            (Variables|Runtime|SetActive%20Battery (.AsItem%20Object%20Consumable%20BASE (Utilities|Casting|CastToItemObject_ConsumableBASE _itemobject)) :!label _label)))
        (:Is%20Not%20Valid
          (goto _label))))))

(event OnItemRemovedfromAttachmentSlot(BP_AttachmentHandler)
  (params (Address :type Slot%20Address%20Structure))
  ;[0.09896 0.09896 0.09896] On Detach Any Item
  (bind _found (CallFunction|TryFindBattery))
  (if (not _found)
    (Variables|Runtime|SetActive%20Battery 0)
    (CallFunction|OnBatteryDead)))

(event Custom|On%20Battery%20Dead
  ;[0.09896 0.09896 0.09896] Try finding another battery if it has multiple battery slots
  (bind _found (CallFunction|TryFindBattery))
  (if (not _found)
    (Variables|Runtime|SetCurrent%20Intensity 0.0)))

(event EventOnItemAttached
  (params (Should%20Hold :type Boolean))
  ;[0.09896 0.09896 0.09896] Hide mesh if it is not held
  (Variables|Default|SetFlashlight%20Is%20Held Should%20Hold) ; Double click for detailed explanation
  (Variables|Runtime|SetIs%20Enabled false))

(event EventDetachfromOwner
  ;[0.09896 0.09896 0.09896] Hide mesh if it is not held
  (|CallParentFunction)
  (Rendering|SetActorHiddenInGame false))

(event EventPrimaryUse
  ;[0.09896 0.09896 0.09896] Use Flashlight
  (bind _output_get (Variables|Runtime|SetIs%20Enabled (not (Variables|Runtime|GetIs%20Enabled))))
  (if _output_get
    (if (CallFunction|HasActiveBattery)
      (Variables|Runtime|SetCurrent%20Intensity (Variables|Parameters|GetFlashlight%20Intensity) :!label _label)
      (if (Utilities|Time|IsValidTimerHandle (Variables|Runtime|GetConsume%20Timer))
        (Utilities|Time|UnpauseTimerbyHandle (Variables|Runtime|GetConsume%20Timer))
        (else
          (bind _returnvalue (Utilities|Time|SetTimerbyEvent (EventDispatchers|CreateEvent :!event ConsumeBattery) (Variables|Parameters|GetBattery%20Update%20Interval) true))
          (Variables|Runtime|SetConsume%20Timer _returnvalue)))
      (else
        (bind _found (CallFunction|TryFindBattery))
        (if _found
          (goto _label))))
    (else
      (Variables|Runtime|SetCurrent%20Intensity 0.0)
      (Utilities|Time|PauseTimerbyHandle (Variables|Runtime|GetConsume%20Timer)))))

(event EventBeginPlay
  ;[0.09896 0.09896 0.09896] BeginPlay
  (|CallParentFunction)
  (Networking|SwitchHasAuthority
    (:Authority
      (CallFunction|TryFindBattery))))

(fn ConstructionScript
  (|CallParentFunction))

(fn HasActiveBattery
  (bind _active_battery (Variables|Runtime|GetActive%20Battery))
  (Utilities|IsValid _active_battery
    (:Is%20Valid
      (if (Default|IsPercentZero _active_battery)
        _
        (else
          (return true))))
    (:Is%20Not%20Valid
      _))
  (return false))

(fn TryFindBattery
  (Utilities|FlowControl|Sequence
    (:then_0
      (for _array_element (Utilities|Struct|BreakItemInfo (Variables|Default|GetItem%20Info))
        (bind _owner_inventory (Variables|Default|GetOwner%20Inventory)
          (:then
            (bind _asitem_object_consumable_base (Utilities|Casting|CastToItemObject_ConsumableBASE (Utilities|Struct|BreakItemInfo (Default|GetItem(copy)byUID _owner_inventory (Utilities|Struct|MakeSlotAddress _array_element)))))
            (if (not (Default|IsPercentZero _asitem_object_consumable_base))
              (Variables|Runtime|SetActive%20Battery _asitem_object_consumable_base)
              (return true)))
          (:else))))
    (:then_1
      (return false))))

(fn OnRepCurrentIntensity
  (Rendering|Components|Light|SetIntensity (Variables|Runtime|GetLight) (Variables|Runtime|GetCurrent%20Intensity)))

(fn ConsumeBattery
  (bind _active_battery (Variables|Runtime|GetActive%20Battery)
    (:then
      (bind _new_percent (Default|ReducePercent _active_battery (* (Variables|Parameters|GetBattery%20Update%20Interval) (Utilities|Time|GetWorldDeltaSeconds) (Variables|Parameters|GetBattery%20Consume%20Multiplier))))
      (|DebugPrintNewPercent _new_percent)
      (if (Default|IsPercentZero (Variables|Runtime|GetActive%20Battery))
        (CallFunction|OnBatteryDead)))
    (:else)))

(fn OnRepFlashlightIsHeld
  ;[0.09896 0.09896 0.09896] Unlike other holdables, the flashlight does not have a secondary socket. Therefore, it hides itself when attached to secondary socket(unequipped).
  (Rendering|SetActorHiddenInGame (not (Variables|Default|GetFlashlight%20Is%20Held))))