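; Inventory attachment item for a weapon suppressor that tells its owning actor when a silencer is fitted or removed.
; Attaching runs the parent logic, then sends SetSilencerReferenceMessage true to the target component's owner.
; Detaching and destruction send false to the item's owner.
; An IsPreviewActor branch keeps preview copies from changing the silencer state.
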(event EventDetachfromOwner
  ;[0.09896 0.09896 0.09896] Set silencer parameters on attach / detach
  (Utilities|IsPreviewActor
    (:false
      (Class|BPIWeaponAGIS|SetSilencerReference(Message) (Components|GetOwner) false))))

(event EventDestroyed
  ;[0.09896 0.09896 0.09896] Set silencer parameters on attach / detach
  (|CallParentFunction)
  (Utilities|IsPreviewActor
    (:false
      (Class|BPIWeaponAGIS|SetSilencerReference(Message) (Components|GetOwner) false))))

(event EventAttachItemtoComponent
  (params (Component :type Scene%20Component%20Object%20Reference) (SocketName :type Name :default "None"))
  ;[0.09896 0.09896 0.09896] Set silencer parameters on attach / detach
  (|CallParentFunction Component SocketName)
  (Utilities|IsPreviewActor
    (:false
      (Class|BPIWeaponAGIS|SetSilencerReference(Message) (Components|GetOwner Component) true))))

(fn ConstructionScript
  (|CallParentFunction))