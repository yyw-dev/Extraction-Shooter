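; Base magazine attachment item that stores a bullet count and exposes functions to query, set and add to it.
; On attach it registers itself with the component owner through a magazine-reference message, and on detach it clears that reference.
; The count persists in an ItemObject_Magazine, read on spawn and written on destroy.
; AddBulletCount writes to the object immediately, while SetBulletCount changes only the local value.
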(event EventWriteItemPropertiestoObject
  ;[0.09896 0.09896 0.09896] Write / read variables from object
  (bind _asitem_object_magazine (Utilities|Casting|CastToItemObject_Magazine (CallFunction|GetItemObject)))
  (Default|SetBulletCountinMagazine _asitem_object_magazine (Variables|Default|GetBullet%20Count)))

(event EventReadItemPropertiesfromObject
  ;[0.09896 0.09896 0.09896] Write / read variables from object
  (bind _asitem_object_magazine (Utilities|Casting|CastToItemObject_Magazine (CallFunction|GetItemObject)))
  (bind _bullet_count (Default|GetBulletCountinMagazine _asitem_object_magazine))
  (Variables|Default|SetBullet%20Count _bullet_count))

(event EventAttachItemtoComponent
  (params (Component :type Scene%20Component%20Object%20Reference) (SocketName :type Name :default "None"))
  ;[0.09896 0.09896 0.09896] Set magazine parameters on attach / detach
  (|CallParentFunction Component SocketName)
  (Class|BPIWeaponAGIS|SetMagazineReference(Message) (Components|GetOwner Component) self))

(event EventDetachfromOwner
  ;[0.09896 0.09896 0.09896] Set magazine parameters on attach / detach
  (Class|BPIWeaponAGIS|SetMagazineReference(Message) (Components|GetOwner)))

(fn ConstructionScript
  (|CallParentFunction))

(fn AddBulletCount
  (params (Amount%20To%20Add :type Integer))
  (Variables|Default|SetBullet%20Count (+ Amount%20To%20Add (Variables|Default|GetBullet%20Count)))
  (CallFunction|WriteItemPropertiestoObject))

(fn GetBulletCount
  (return (Variables|Default|GetBullet%20Count)))

(fn SetBulletCount
  (params (Bullet%20Count :type Integer))
  (Variables|Default|SetBullet%20Count Bullet%20Count))

(fn HasBullet
  (return (> (Variables|Default|GetBullet%20Count) 0)))