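; Rifle flashlight attachment item whose spotlight toggles on primary use and runs on battery items slotted into it.
; While lit, a looping timer runs, paused when switched off, and battery consumption lowers the active battery's percent.
; Attach, detach and depletion events select a charged battery from the item's own containers or zero the intensity.
; CurrentIntensity drives the spotlight through its OnRep function.
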(event OnItemAddedtoAttachmentSlot(BP_AttachmentHandler)
  (params (Added%20Item :type Item%20Info%20Structure))
  (bind (_itemid _itemobject) (Utilities|Struct|BreakItemInfo Added%20Item))
  ;[0.09896 0.09896 0.09896] On Attach Battery
  (if (not (CallFunction|IsPreviewActor))
    (if (== _itemid (Utilities|Struct|BreakDataTableRowHandle (Variables|Parameters|GetBattery%20Item))) ; Is it battery?
      (Utilities|IsValid (Variables|Runtime|GetActive%20Battery) ; Is there already battery attached?
        (:Is%20Valid
          (if (Default|IsPercentZero (Variables|Runtime|GetActive%20Battery)) ; is already attached battery 0 percent?
            (Variables|Runtime|SetActive%20Battery (.AsItem%20Object%20Consumable%20BASE (Utilities|Casting|CastToItemObject_ConsumableBASE _itemobject)) :!label _label)))
        (:Is%20Not%20Valid
          (goto _label))))))

(event OnItemRemovedfromAttachmentSlot(BP_AttachmentHandler)
  (params (Address :type Slot%20Address%20Structure))
  ;[0.09896 0.09896 0.09896] On Detach Any Item
  (bind _found (CallFunction|TryFindBattery))
  (if (not _found)
    (Variables|Runtime|SetActive%20Battery 0)
    (CallFunction|OnBatteryDead)))

(event Custom|On%20Battery%20Dead
  (Variables|Runtime|SetCurrent%20Intensity 0.0)
  (CallFunction|TryFindBattery))

(event Custom|Update%20Light%20Intensity
  ;[0.09896 0.09896 0.09896] Update  Light Intensity
  (if (Variables|Runtime|GetIs%20Enabled)
    (if (CallFunction|HasActiveBattery)
      (Variables|Runtime|SetCurrent%20Intensity (Variables|Parameters|GetFlashlight%20Intensity) :!label _label)
      (if (Utilities|Time|IsValidTimerHandle (Variables|Runtime|GetConsume%20Timer))
        (Utilities|Time|UnpauseTimerbyHandle (Variables|Runtime|GetConsume%20Timer))
        (else
          (bind _returnvalue (Utilities|Time|SetTimerbyEvent (EventDispatchers|CreateEvent :!event ConsumeBattery) (Variables|Parameters|GetBattery%20Update%20Interval) true))
          (Variables|Runtime|SetConsume%20Timer _returnvalue)))
      (else
        (bind _found (CallFunction|TryFindBattery))
        (if _found
          (goto _label))))
    (else
      (Variables|Runtime|SetCurrent%20Intensity 0.0)
      (Utilities|Time|PauseTimerbyHandle (Variables|Runtime|GetConsume%20Timer)))))

(event EventPrimaryUse
  ;[0.09896 0.09896 0.09896] Use Flashlight
  (Variables|Runtime|SetIs%20Enabled (not (Variables|Runtime|GetIs%20Enabled)))
  (CallFunction|UpdateLightIntensity))

(event EventBeginPlay
  (|CallParentFunction)
  (Networking|SwitchHasAuthority
    (:Authority
      (CallFunction|UpdateLightIntensity))))

(fn ConstructionScript
  (|CallParentFunction))

(fn HasActiveBattery
  (bind _active_battery (Variables|Runtime|GetActive%20Battery))
  (Utilities|IsValid _active_battery
    (:Is%20Valid
      (if (Default|IsPercentZero _active_battery)
        _
        (else
          (return true))))
    (:Is%20Not%20Valid
      _))
  (return false))

(fn OnRepCurrentIntensity
  (Rendering|Components|Light|SetIntensity (Variables|Default|GetSpotLight) (Variables|Runtime|GetCurrent%20Intensity)))

(fn TryFindBattery
  (Utilities|FlowControl|Sequence
    (:then_0
      (for _array_element (Utilities|Struct|BreakItemInfo (Variables|Default|GetItem%20Info))
        (bind _asitem_object_consumable_base (Utilities|Casting|CastToItemObject_ConsumableBASE (Utilities|Struct|BreakItemInfo (Default|GetItem(copy)byUID (Variables|/Game/INVENTORY/Core/BP_AttachmentHandler.BP_AttachmentHandler_C|GetParent%20Inventory (Variables|Default|GetBP_AttachmentHandler)) (Utilities|Struct|MakeSlotAddress _array_element)))))
        (if (not (Default|IsPercentZero _asitem_object_consumable_base))
          (Variables|Runtime|SetActive%20Battery _asitem_object_consumable_base)
          (return true))))
    (:then_1
      (return false))))

(fn ConsumeBattery
  (Utilities|FlowControl|Sequence
    (:then_0
      (bind _active_battery (Variables|Runtime|GetActive%20Battery)
        (:then
          (bind _new_percent (Default|ReducePercent _active_battery (|CalculateConsumeAmount)))
          (|DebugPrintNewPercent _new_percent))
        (:else)))
    (:then_1
      (bind _active_battery_2 (Variables|Runtime|GetActive%20Battery)
        (:then
          (if (Default|IsPercentZero _active_battery_2)
            (CallFunction|OnBatteryDead)))
        (:else)))))