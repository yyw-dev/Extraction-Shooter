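; BP_Generator is an interactable generator that runs on consumable items placed in its equipper inventory, opened on interact.
; The server listens for slot updates and sets replicated Running while the item has percent left, clearing it on empty.
; OnRep_Running drives a looping Shake timer that both jitters the mesh and drains the item, broadcasting remaining fuel.
; Tracing the generator toggles a mesh outline.
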(event Custom|OnSlotUpdated_Event
  (params (Inventory :type Inventory%20Main%20Object%20Reference) (Address :type Slot%20Address%20Structure) (New%20Item :type Item%20Info%20Structure))
  (bind (_itemid _itemobject) (Utilities|Struct|BreakItemInfo New%20Item))
  ;[0.09896 0.09896 0.09896] Listen Inventory to change color when card equipped
  (Utilities|IsValidName _itemid
    (:Valid
      (bind _asitem_object_consumable_base (Utilities|Casting|CastToItemObject_ConsumableBASE _itemobject))
      (Variables|Default|SetRunning (not (Default|IsPercentZero _asitem_object_consumable_base)))
      (bind _output_get (Variables|Default|SetCurrent%20Item%20Data _asitem_object_consumable_base))
      (EventDispatchers|AssignOnPercentZero _output_get (delegate Custom|On%20Percent%20Zero_Event)))
    (:Not%20Valid
      (Variables|Default|SetRunning false)
      (CallFunction|SetRemainedFuel 0.0))))

(event Custom|Shake
  (bind _returnvalue (Math|Random|RandomFloatinRange -1.0 1.0))
  ;[0.09896 0.09896 0.09896] Shake when fuel equipped
  (Transformation|SetRelativeLocation (Variables|Default|GetGeneratorMesh) (Math|Vector|MakeVector _returnvalue _returnvalue (Math|Random|RandomFloatinRange 0.0 2.0)) false false)
  (bind _current_item_data (Variables|Default|GetCurrent%20Item%20Data)
    (:then
      (bind _new_percent (Default|ReducePercent _current_item_data 0.0032))
      (CallFunction|SetRemainedFuel _new_percent))
    (:else)))

(event Custom|On%20Percent%20Zero_Event
  ;[0.09896 0.09896 0.09896] Listen Inventory to change color when card equipped
  (Variables|Default|SetRunning false))

(event EventBeginPlay
  ;[0.09896 0.09896 0.09896] Listen Inventory to change color when card equipped
  (Networking|SwitchHasAuthority
    (:Authority
      (EventDispatchers|AssignOnSlotUpdatedSERVER (Variables|Default|GetIC_Equipper) (delegate Custom|OnSlotUpdated_Event)))))

(event EventOnTraceLeave
  ;[0.09896 0.09896 0.09896] Interaction
  (Utilities|OutlineonTrace (Variables|Default|GetGeneratorMesh)) ; enters at On Trace Leave
)

(event EventOnTraceEnter
  ;[0.09896 0.09896 0.09896] Interaction
  (Utilities|OutlineonTrace (Variables|Default|GetGeneratorMesh)))

(event EventOnInteract
  (params (Inventory%20C :type Inventory%20Player%20Object%20Reference) (Interaction :type EInteractionType%20Enum :default "NewEnumerator5"))
  ;[0.09896 0.09896 0.09896] Interaction
  (Default|ListenInventory Inventory%20C (Variables|Default|GetIC_Equipper)))

(fn ConstructionScript)

(fn OnRepRunning
  (if (Variables|Default|GetRunning)
    (Utilities|Time|SetTimerbyFunctionName 0 "Shake" 0.03 true)
    (else
      (Utilities|Time|ClearTimerbyFunctionName 0 "Shake")
      (Transformation|SetRelativeLocation (Variables|Default|GetGeneratorMesh) "0, 0, 0" false false))))

(fn SetRemainedFuel
  (params (Remained%20Fuel :type Float%20%28double-precision%29))
  (bind _output_get (Variables|Default|SetRemained%20Fuel Remained%20Fuel))
  (Default|CallOnFuelUpdate _output_get))

(fn GetTracePoint
  (return "0, 0, 0" "0, 0, 0"))