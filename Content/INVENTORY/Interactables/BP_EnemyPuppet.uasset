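; BP_EnemyPuppet is an enemy that takes damage and becomes an interactable inventory once dead.
; Point damage is forwarded to its CombatComponent, whose IsDead flag gates all interaction.
; When dead, interacting makes the interactor's inventory component listen to the puppet's ICHuman inventory, and trace enter and leave toggle a mesh outline through outlineOnTrace.
; GetTracePoint is a stub returning zero vectors.
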(event EventOnInteract
  (params (Inventory%20C :type Inventory%20Player%20Object%20Reference) (Interaction :type EInteractionType%20Enum :default "NewEnumerator5"))
  ;[0.09896 0.09896 0.09896] Interaction
  (if (CallFunction|IsDead)
    (Default|ListenInventory Inventory%20C (Variables|Default|GetIC_Human))))

(event EventOnTraceEnter
  ;[0.09896 0.09896 0.09896] Interaction
  (if (CallFunction|IsDead)
    (Utilities|OutlineonTrace (Variables|Character|GetMesh))))

(event EventOnTraceLeave
  ;[0.09896 0.09896 0.09896] Interaction
  (if (CallFunction|IsDead)
    (Utilities|OutlineonTrace (Variables|Character|GetMesh)) ; enters at On Trace Leave
  ))

(event Game|Damage|EventPointDamage
  (params (Damage :type Float%20%28single-precision%29) (DamageType :type Damage%20Type%20Object%20Reference) (HitLocation :type Vector :default "0, 0, 0") (HitNormal :type Vector :default "0, 0, 0") (HitComponent :type Primitive%20Component%20Object%20Reference) (BoneName :type Name :default "None") (ShotFromDirection :type Vector :default "0, 0, 0") (InstigatedBy :type Controller%20Object%20Reference) (DamageCauser :type Actor%20Object%20Reference) (HitInfo :type Hit%20Result%20Structure%20%28by%20ref%29))
  ;[0.09896 0.09896 0.09896] Take Damage
  (Default|TakeDamage (Variables|Default|GetCombatComponent) Damage DamageCauser InstigatedBy HitLocation HitNormal))

(fn ConstructionScript)

(fn IsDead
  (return (Variables|/Game/INVENTORY/Core/CombatComponent.CombatComponent_C|GetIs%20Dead (Variables|Default|GetCombatComponent))))

(fn GetTracePoint
  (return "0, 0, 0" "0, 0, 0"))