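; A two-panel sliding door that opens and closes in response to items placed in another actor's inventory.
; On the server, it caches panel positions and binds to slot updates from the inventory component of ActorToListen.
; An added item plays a timeline that lerps the panels apart, unless it is a depleted consumable.
; Item removal or a consumable's percent-zero event reverses the timeline to close the door.
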(event Custom|OnSlotUpdated
  (params (Inventory :type Inventory%20Main%20Object%20Reference) (Address :type Slot%20Address%20Structure) (New%20Item :type Item%20Info%20Structure))
  (bind (_itemid _itemobject) (Utilities|Struct|BreakItemInfo New%20Item))
  ;[0.09896 0.09896 0.09896] Listen inventory and animate door
  (Utilities|FlowControl|Sequence
    (:then_0
      (Utilities|IsValidName _itemid ; Valid - Item Added\nNot Valid - Item Removed
        (:Valid
          (bind _asitem_object_consumable (Utilities|Casting|CastToItemObject_ConsumableBASE _itemobject)
            (:then
              (if (not (Default|IsPercentZero _asitem_object_consumable))
                (bind _alpha (Timeline|Door%20TL Play)
                  (:Update
                    (Transformation|SetRelativeLocation (Variables|Default|GetLeft) (Math|Vector|Lerp(Vector) (Variables|Default|GetLeft%20Door%20Initial%20Pos) (Variables|Default|GetLeft%20Door%20Opened%20Pos) _alpha) false false)
                    (Transformation|SetRelativeLocation (Variables|Default|GetRight) (Math|Vector|Lerp(Vector) (Variables|Default|GetRight%20Door%20Initial%20Pos) (Variables|Default|GetRight%20Door%20Opened%20Pos) _alpha) false false)))))
            (:CastFailed
              (Timeline|Door%20TL Play))))
        (:Not%20Valid
          (Timeline|Door%20TL Reverse))))
    (:then_1
      (bind _asitem_object_consumable_2 (Utilities|Casting|CastToItemObject_ConsumableBASE _itemobject))
      (EventDispatchers|AssignOnPercentZero _asitem_object_consumable_2 (delegate Custom|On%20Percent%20Zero_Event)))))

(event Custom|On%20Percent%20Zero_Event
  ;[0.09896 0.09896 0.09896] Listen inventory and animate door
  (bind _alpha (Timeline|Door%20TL Reverse)
    (:Update
      (Transformation|SetRelativeLocation (Variables|Default|GetLeft) (Math|Vector|Lerp(Vector) (Variables|Default|GetLeft%20Door%20Initial%20Pos) (Variables|Default|GetLeft%20Door%20Opened%20Pos) _alpha) false false)
      (Transformation|SetRelativeLocation (Variables|Default|GetRight) (Math|Vector|Lerp(Vector) (Variables|Default|GetRight%20Door%20Initial%20Pos) (Variables|Default|GetRight%20Door%20Opened%20Pos) _alpha) false false))))

(event EventBeginPlay
  ;[0.09896 0.09896 0.09896] Listen inventory and animate door
  (Networking|SwitchHasAuthority
    (:Authority
      (Utilities|FlowControl|Sequence
        (:then_0
          ;[0.09896 0.09896 0.09896] Set Variables
          (bind _output_get (Variables|Default|SetLeft%20Door%20Initial%20Pos (Variables|/Script/Engine.SceneComponent|GetRelativeLocation (Variables|Default|GetLeft))))
          (Variables|Default|SetLeft%20Door%20Opened%20Pos (+ _output_get "-100.000000,0.000000,0.000000"))
          (bind _output_get_2 (Variables|Default|SetRight%20Door%20Initial%20Pos (Variables|/Script/Engine.SceneComponent|GetRelativeLocation (Variables|Default|GetRight))))
          (Variables|Default|SetRight%20Door%20Opened%20Pos (+ _output_get_2 "100.000000,0.000000,0.000000")))
        (:then_1
          (bind _actor_to_listen (Variables|Default|GetActor%20to%20Listen)
            (:then
              (bind _output_get_3 (Variables|Default|SetListening%20Inventory (Actor|GetComponentbyClass _actor_to_listen "/Game/INVENTORY/Core/Inventory__Main.Inventory__Main_C")))
              (Utilities|IsValid _output_get_3
                (:Is%20Valid
                  (EventDispatchers|BindEventtoOnSlotUpdatedSERVER _output_get_3 (delegate Custom|OnSlotUpdated)))))
            (:else)))))))

(fn ConstructionScript)