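; Keycard reader interactable whose indicator turns green while an item sits in its equipper slot and red otherwise.
; The server listens to ICEquipper slot updates and sets replicated HasItem from item validity, whose OnRep swaps the ReaderMesh emissive material.
; Interacting makes the player's inventory component listen to ICEquipper, and trace enter and leave toggle the outline highlight.
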(event Custom|OnSlotUpdated_Event
  (params (Inventory :type Inventory%20Main%20Object%20Reference) (Address :type Slot%20Address%20Structure) (New%20Item :type Item%20Info%20Structure))
  ;[0.09896 0.09896 0.09896] Listen Inventory to change color when card equipped
  (Variables|Default|SetHasItem (CallFunction|IsValidItem New%20Item)))

(event EventBeginPlay
  ;[0.09896 0.09896 0.09896] Listen Inventory to change color when card equipped
  (Networking|SwitchHasAuthority
    (:Authority
      (EventDispatchers|AssignOnSlotUpdatedSERVER (Variables|Default|GetIC_Equipper) (delegate Custom|OnSlotUpdated_Event)))))

(event EventOnTraceLeave
  ;[0.09896 0.09896 0.09896] Interaction
  (Utilities|OutlineonTrace (Variables|Default|GetReaderMesh)) ; enters at On Trace Leave
)

(event EventOnTraceEnter
  ;[0.09896 0.09896 0.09896] Interaction
  (Utilities|OutlineonTrace (Variables|Default|GetReaderMesh)))

(event EventOnInteract
  (params (Inventory%20C :type Inventory%20Player%20Object%20Reference) (Interaction :type EInteractionType%20Enum :default "NewEnumerator5"))
  ;[0.09896 0.09896 0.09896] Interaction
  (Default|ListenInventory Inventory%20C (Variables|Default|GetIC_Equipper)))

(fn ConstructionScript)

(fn OnRepHasItem
  (Rendering|Material|SetMaterial (Variables|Default|GetReaderMesh) 3 (select (Variables|Default|GetHasItem) "/Game/INVENTORY/Other/Materials/MI_GreenEmissive.MI_GreenEmissive" "/Game/INVENTORY/Other/Materials/MI_RedEmissive.MI_RedEmissive")))

(fn GetTracePoint
  (return "0, 0, 0" "0, 0, 0"))