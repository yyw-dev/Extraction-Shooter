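; BP_Smelter is an interactable smelter that opens its crafting inventory when the player interacts with it.
; Interaction makes the player's inventory component listen to InventoryCrafting, and trace enter/leave events toggle an outline on the mesh.
; Fuel status is read one tick after BeginPlay and updated by the crafting component's change event.
; The RepNotify HasFuel variable shows or hides the point light to match.
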(event OnFuelStatusChanged(Inventory_Crafting)
  (params (Has%20Fuel :type Boolean))
  ;[0.09896 0.09896 0.09896] Toggle Light
  (Variables|Default|SetHas%20Fuel Has%20Fuel))

(event EventBeginPlay
  ;[0.09896 0.09896 0.09896] Toggle Light
  (Utilities|FlowControl|DelayUntilNextTick)
  (Variables|Default|SetHas%20Fuel (Default|GetFuelStatus (Variables|Default|GetInventory_Crafting))))

(event EventOnInteract
  (params (Inventory%20C :type Inventory%20Player%20Object%20Reference) (Interaction :type EInteractionType%20Enum :default "NewEnumerator5"))
  ;[0.09896 0.09896 0.09896] Interaction
  (Default|ListenInventory Inventory%20C (Variables|Default|GetInventory_Crafting)))

(event EventOnTraceEnter
  ;[0.09896 0.09896 0.09896] Interaction
  (Utilities|OutlineonTrace (Variables|Default|GetStaticMesh)))

(event EventOnTraceLeave
  ;[0.09896 0.09896 0.09896] Interaction
  (Utilities|OutlineonTrace (Variables|Default|GetStaticMesh)) ; enters at On Trace Leave
)

(fn ConstructionScript)

(fn OnRepHasFuel
  (Development|SetHiddeninGame (Variables|Default|GetPointLight) (not (Variables|Default|GetHas%20Fuel)) false))

(fn GetTracePoint
  (return "0, 0, 0" "0, 0, 0"))