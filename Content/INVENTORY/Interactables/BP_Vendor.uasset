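; BP_Vendor is an interactable NPC vendor that carries its own inventory component.
; On interaction, it passes that vendor inventory to the interacting inventory component through ListenInventory.
; Trace enter and leave events toggle an outline on its skeletal mesh through the outlineOnTrace helper.
; The construction script shows the NPC name on a text render, while GetTracePoint returns only zero vectors.
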(event EventOnTraceLeave
  ;[0.09896 0.09896 0.09896] Interaction
  (Utilities|OutlineonTrace (Variables|Default|GetSkeletalMesh)) ; enters at On Trace Leave
)

(event EventOnTraceEnter
  ;[0.09896 0.09896 0.09896] Interaction
  (Utilities|OutlineonTrace (Variables|Default|GetSkeletalMesh)))

(event EventOnInteract
  (params (Inventory%20C :type Inventory%20Player%20Object%20Reference) (Interaction :type EInteractionType%20Enum :default "NewEnumerator5"))
  ;[0.09896 0.09896 0.09896] Interaction
  (Default|ListenInventory Inventory%20C (Variables|Default|GetIC_Vendor)))

(fn ConstructionScript
  (Rendering|Components|TextRender|SetText (Variables|Default|GetTextRender) (Variables|Default|GetNPC%20Name)))

(fn GetTracePoint
  (return "0, 0, 0" "0, 0, 0"))